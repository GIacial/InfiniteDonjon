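; PC_Prete is a player combatant class Blueprint that defines the "Prête" class, equipped with a healing staff.
; Its construction script runs the parent's, then sets hardcoded primary stats, two secondary stats and the Equipement_Heal_Staff weapon.
; It overrides GetClassName to return the display name and adds no event logic of its own.
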(fn `getClassName`
  (returns (ClassName :type Name))
  (return "Prête"))

(fn `UserConstructionScript`
  (`parent.UserConstructionScript`)
  (`self.SetPrimaryStat` 59 "NewEnumerator0")
  (`self.SetPrimaryStat` 70 "NewEnumerator1")
  (`self.SetPrimaryStat` 68 "NewEnumerator2")
  (`self.SetPrimaryStat` 75 "NewEnumerator3")
  (`self.SetPrimaryStat` 65 "NewEnumerator4")
  (`self.SetPrimaryStat` 72 "NewEnumerator5")
  (`self.SetPrimaryStat` 75 "NewEnumerator6")
  (`self.SetPrimaryStat` 70 "NewEnumerator7")
  (`self.SetSecondaryStat` "NewEnumerator3" 2)
  (`self.SetSecondaryStat` "NewEnumerator2" 1)
  (`self.setArme` "/Game/Class/Equipement/Stuff/Staff/Equipement_Heal_Staff.Equipement_Heal_Staff_C"))