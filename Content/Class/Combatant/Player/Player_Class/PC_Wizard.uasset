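; PC_Wizard is the Wizard player class, a child combatant Blueprint that reports its class name as "Sorcier".
; Its construction script runs the parent's, then sets eight primary stats and one secondary stat and assigns a sorcerer staff as the weapon.
; It overrides the class name getter without calling the parent, and its event graph holds only disabled default events.
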(fn `getClassName`
  (returns (ClassName :type Name))
  (return "Sorcier"))

(fn `UserConstructionScript`
  (`parent.UserConstructionScript`)
  (`self.SetPrimaryStat` 51 "NewEnumerator0")
  (`self.SetPrimaryStat` 75 "NewEnumerator1")
  (`self.SetPrimaryStat` 65 "NewEnumerator2")
  (`self.SetPrimaryStat` 80 "NewEnumerator3")
  (`self.SetPrimaryStat` 75 "NewEnumerator4")
  (`self.SetPrimaryStat` 68 "NewEnumerator5")
  (`self.SetPrimaryStat` 65 "NewEnumerator6")
  (`self.SetPrimaryStat` 75 "NewEnumerator7")
  (`self.SetSecondaryStat` "NewEnumerator3" 3)
  (`self.setArme` "/Game/Class/Equipement/Stuff/Staff/Equipement_Staff_sorcier.Equipement_Staff_sorcier_C"))