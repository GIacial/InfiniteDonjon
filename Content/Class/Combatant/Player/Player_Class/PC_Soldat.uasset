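; Player class Blueprint for the "Soldat" (soldier) combatant, defining its stats and weapon.
; The construction script runs the parent's setup, then sets eight primary stats and one secondary stat and equips a wooden sword.
; GetClassName overrides the parent to return the class name, and the event graph holds no active logic.
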(fn `getClassName`
  (returns (ClassName :type Name))
  (return "Soldat"))

(fn `UserConstructionScript`
  (`parent.UserConstructionScript`)
  (`self.SetPrimaryStat` 80 "NewEnumerator0")
  (`self.SetPrimaryStat` 70 "NewEnumerator1")
  (`self.SetPrimaryStat` 78 "NewEnumerator2")
  (`self.SetPrimaryStat` 50 "NewEnumerator3")
  (`self.SetPrimaryStat` 65 "NewEnumerator4")
  (`self.SetPrimaryStat` 75 "NewEnumerator5")
  (`self.SetPrimaryStat` 68 "NewEnumerator6")
  (`self.SetPrimaryStat` 68 "NewEnumerator7")
  (`self.SetSecondaryStat` "NewEnumerator2" 3)
  (`self.setArme` "/Game/Class/Equipement/Stuff/Sword/Equipement_Wodden_Sword.Equipement_Wodden_Sword_C"))